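; Zombie enemy Blueprint that reacts to the player's parry by driving state in its animation Blueprint.
; BeginPlay caches the skeletal mesh's anim instance as ABP_Zombie.
; Each Tick polls the first player state's parry flag and sets the anim instance's IsParried only while IsParriable is also true, clearing it otherwise.
; Both outcomes print a debug string every frame.
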(event `self.ReceiveTick`
  (params (DeltaSeconds :type "Float (single-precision)"))
  (bind _as_abp_zombie (`self.As ABP Zombie`))
  ;[1 1 1] If player is parrying
  (bind _isparried (message `/Game/Custom/Parry/BPI_PlayerStateInterface.GetIsParried` (`GameplayStatics.GetPlayerState` 0)))
  (if (and _isparried (`/Game/Custom/Parry/ABP_Zombie.IsParriable` _as_abp_zombie))
    (`KismetSystemLibrary.PrintString` "does parry!")
    (set `/Game/Custom/Parry/ABP_Zombie.IsParried` true _as_abp_zombie)
    (else
      (`KismetSystemLibrary.PrintString` "doesn't parry :(")
      (set `/Game/Custom/Parry/ABP_Zombie.IsParried` false _as_abp_zombie))))

(event `self.ReceiveBeginPlay`
  (bind _asabp_zombie (cast `/Game/Custom/Parry/ABP_Zombie` (`SkeletalMeshComponent.GetAnimInstance` (`self.SkeletalMesh`))))
  ;[1 1 1] If zombie is parryable
  (set `self.As ABP Zombie` _asabp_zombie))

(fn `UserConstructionScript`)