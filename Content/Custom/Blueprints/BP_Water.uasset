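; Water volume actor that applies buoyancy to actors overlapping its Box, with the Water component placed at WaterLevel on BeginPlay.
; Box overlap events maintain the Actors list, which Tick loops through.
; Submerged volume is estimated as bounds footprint times depth below WaterLevel, without clamping to object height.
; An upward Archimedes force, scaled by Density and DeltaSeconds, is applied to each static mesh at the actor location.
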(event `self.ReceiveBeginPlay`
  (`SceneComponent.K2_SetRelativeLocation` (`self.Water`) (`KismetMathLibrary.MakeVector` 0.0 0.0 (`self.WaterLevel`)) false false))

(event `self.Box.OnComponentBeginOverlap`
  (params (OverlappedComponent :type "PrimitiveComponent Object Reference") (OtherActor :type "Actor Object Reference") (OtherComp :type "PrimitiveComponent Object Reference") (OtherBodyIndex :type Integer) (bFromSweep :type Boolean) (SweepResult :type "HitResult Structure (by ref)"))
  (`KismetArrayLibrary.Array_AddUnique` (`self.Actors`) OtherActor))

(event `self.Box.OnComponentEndOverlap`
  (params (OverlappedComponent :type "PrimitiveComponent Object Reference") (OtherActor :type "Actor Object Reference") (OtherComp :type "PrimitiveComponent Object Reference") (OtherBodyIndex :type Integer))
  (`KismetArrayLibrary.Array_RemoveItem` (`self.Actors`) OtherActor))

(event `self.ReceiveTick`
  (params (DeltaSeconds :type "Float (single-precision)"))
  (for _array_element (`self.Actors`)
    (bind (_origin _boxextent) (`self.GetActorBounds` _array_element false false))
    (bind _output_get (set `self.SubVolume` (* (- (`self.WaterLevel`) (- (.z _origin) (.z _boxextent))) (* (* (.x _boxextent) (.y _boxextent)) 4.0))))
    (bind _returnvalue (* (* (`self.Density`) _output_get) 9.8))
    (if (not (< _returnvalue 0.1))
      (`PrimitiveComponent.AddForceAtLocation` (`self.GetComponentByClass` _array_element "/Script/Engine.StaticMeshComponent") (* (* _returnvalue DeltaSeconds) (`KismetMathLibrary.GetUpVector` (struct))) (`self.K2_GetActorLocation` _array_element) "None"))))

(fn `UserConstructionScript`)