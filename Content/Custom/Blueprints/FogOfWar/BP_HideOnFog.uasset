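; BP_HideOnFog is a fog-of-war actor whose mesh fades its visibility as fog volumes affect it.
; UpdateFogVolumeAndSetVisibilityState keeps a running volume count and calls FogTransition only when the count crosses between zero and positive.
; FogTransition plays a timeline forward for a positive count or reverses it otherwise, driving VisibilityIntensity on a dynamic material instance created at BeginPlay.
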(event `self.ReceiveBeginPlay`
  (bind _returnvalue (`PrimitiveComponent.CreateDynamicMaterialInstance` (`self.SM`) 0 null "None"))
  (set `self.DynMatInst` _returnvalue))

(event `FogTransition`
  (params (Show :type Boolean))
  (if Show
    (bind (_direction _alpha) (`Timeline|T_TransitionFog` :!label _label)
      (:`Update`
        (`MaterialInstanceDynamic.SetScalarParameterValue` (`self.DynMatInst`) "VisibilityIntensity" _alpha)))
    (else
      (goto _label :!via `Reverse`))))

(fn `UpdateFogVolumeAndSetVisibilityState`
  (params (VolumeCount :type Integer))
  (bind _output_get (set `self.VolumeFogCounter` (+ (`self.VolumeFogCounter`) VolumeCount)))
  (bind _returnvalue (not (<= _output_get 0)))
  (if (!= _returnvalue (`self.ShowTransition`))
    (`self.FogTransition` _returnvalue)
    (set `self.ShowTransition` _returnvalue)))

(fn `UserConstructionScript`)