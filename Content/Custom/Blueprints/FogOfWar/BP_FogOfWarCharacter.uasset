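; BP_FogOfWarCharacter is a character Blueprint that reveals and hides fog-of-war actors within its sight.
; Two volumes, SeeVolumeFront and SeeVolumeNear, act as the vision area, reacting only to BP_HideOnFog actors.
; Begin and end overlaps send +1 and -1 to each actor's UpdateFogVolumeAndSetVisibilityState, apparently counting covering volumes so visibility holds while any volume still overlaps.
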(event `self.SeeVolumeFront.OnComponentBeginOverlap`
  (params (OverlappedComponent :type "PrimitiveComponent Object Reference") (OtherActor :type "Actor Object Reference") (OtherComp :type "PrimitiveComponent Object Reference") (OtherBodyIndex :type Integer) (bFromSweep :type Boolean) (SweepResult :type "HitResult Structure (by ref)"))
  ;[1 1 1] Show/Hide actor
  ;;[1 1 1] Show
  (bind _asbp_hide_on_fog (cast `/Game/Custom/Blueprints/FogOfWar/BP_HideOnFog` OtherActor))
  (`/Game/Custom/Blueprints/FogOfWar/BP_HideOnFog.UpdateFogVolumeAndSetVisibilityState` _asbp_hide_on_fog 1))

(event `self.SeeVolumeNear.OnComponentBeginOverlap`
  (params (OverlappedComponent :type "PrimitiveComponent Object Reference") (OtherActor :type "Actor Object Reference") (OtherComp :type "PrimitiveComponent Object Reference") (OtherBodyIndex :type Integer) (bFromSweep :type Boolean) (SweepResult :type "HitResult Structure (by ref)"))
  ;[1 1 1] Show/Hide actor
  ;;[1 1 1] Show
  (bind _asbp_hide_on_fog (cast `/Game/Custom/Blueprints/FogOfWar/BP_HideOnFog` OtherActor))
  (`/Game/Custom/Blueprints/FogOfWar/BP_HideOnFog.UpdateFogVolumeAndSetVisibilityState` _asbp_hide_on_fog 1))

(event `self.SeeVolumeNear.OnComponentEndOverlap`
  (params (OverlappedComponent :type "PrimitiveComponent Object Reference") (OtherActor :type "Actor Object Reference") (OtherComp :type "PrimitiveComponent Object Reference") (OtherBodyIndex :type Integer))
  ;[1 1 1] Show/Hide actor
  ;;[1 1 1] Hide
  (bind _asbp_hide_on_fog (cast `/Game/Custom/Blueprints/FogOfWar/BP_HideOnFog` OtherActor))
  (`/Game/Custom/Blueprints/FogOfWar/BP_HideOnFog.UpdateFogVolumeAndSetVisibilityState` _asbp_hide_on_fog -1))

(event `self.SeeVolumeFront.OnComponentEndOverlap`
  (params (OverlappedComponent :type "PrimitiveComponent Object Reference") (OtherActor :type "Actor Object Reference") (OtherComp :type "PrimitiveComponent Object Reference") (OtherBodyIndex :type Integer))
  ;[1 1 1] Show/Hide actor
  ;;[1 1 1] Hide
  (bind _asbp_hide_on_fog (cast `/Game/Custom/Blueprints/FogOfWar/BP_HideOnFog` OtherActor))
  (`/Game/Custom/Blueprints/FogOfWar/BP_HideOnFog.UpdateFogVolumeAndSetVisibilityState` _asbp_hide_on_fog -1))

(fn `UserConstructionScript`
  (`parent.UserConstructionScript`))