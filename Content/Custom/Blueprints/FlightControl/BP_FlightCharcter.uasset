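; Player flight Blueprint that flies a physics-driven static mesh with keyboard throttle, pitch and roll.
; Debug key events set increments that Tick turns into a clamped speed scale, forward physics velocity and rotation changes.
; Pitch and roll compose as quaternion deltas around the actor's own right and forward axes, with no yaw input.
; Each frame updates the flight UI widget created at BeginPlay and feeds speed to a Niagara trail.
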(event EventBeginPlay
  (bind _returnvalue (UserInterface|CreateWidget "/Game/Custom/Blueprints/FlightControl/ui/WBP_FlightUI.WBP_FlightUI_C"))
  (bind _output_get (Variables|Default|SetUI _returnvalue))
  (UserInterface|Viewport|AddtoViewport _output_get 0))

(event Collision|EventActorBeginOverlap
  (params (OtherActor :type Actor%20Object%20Reference)))

(event EventTick
  (params (DeltaSeconds :type Float%20%28single-precision%29))
  (Variables|Default|SetDelta%20Seconds DeltaSeconds)
  (Variables|Default|SetSpeedScale (Math|Float|Clamp(Float) (+ (* (* (Variables|Default|GetDelta%20Seconds) 0.2) (Variables|Default|GetIncrement)) (Variables|Default|GetSpeedScale))))
  (Variables|Default|SetCurrentSpeed (* (Variables|Default|GetMaxSpeed) (Variables|Default|GetSpeedScale)))
  (Physics|SetPhysicsLinearVelocity (Variables|Default|GetStaticMesh) (* (Math|Vector|GetForwardVector (Variables|Default|GetStaticMesh)) (* (Variables|Default|GetMaxSpeed) (Variables|Default|GetSpeedScale))) false "None")
  (Variables|Default|SetPitchAngle (+ (* (Variables|Default|GetPitchIncrement) (Variables|Default|GetDelta%20Seconds) 1e+02) (Variables|Default|GetPitchAngle)))
  (Variables|Default|SetDeltaPitchQuat (Math|Conversions|ToQuaternion(Rotator) (Math|Vector|RotatorfromAxisandAngle (Transformation|GetActorRightVector) (* (Variables|Default|GetPitchIncrement) (Variables|Default|GetDelta%20Seconds) 1e+02))))
  (Variables|Default|SetRollAngle (+ (Variables|Default|GetRollAngle) (* (Variables|Default|GetRollIncrement) (Variables|Default|GetDelta%20Seconds) 1e+02)))
  (Variables|Default|SetDeltaRollQuat (Math|Conversions|ToQuaternion(Rotator) (Math|Vector|RotatorfromAxisandAngle (Transformation|GetActorForwardVector) (* (Variables|Default|GetRollIncrement) (Variables|Default|GetDelta%20Seconds) 1e+02))))
  (Variables|Default|SetCurrentQuat (Math|Conversions|ToQuaternion(Rotator) (Transformation|GetActorRotation)))
  (Transformation|SetActorRotation (Class|KismetMathLibrary|QuatRotator (* (* (Variables|Default|GetDeltaRollQuat) (Variables|Default|GetDeltaPitchQuat)) (Variables|Default|GetCurrentQuat))))
  (Default|UpdateValue (Variables|Default|GetUI) (Variables|Default|GetRollAngle) (Variables|Default|GetPitchAngle) (Variables|Default|GetCurrentSpeed))
  (Effects|Components|ParticleSystem|SetFloatParameter (Variables|Default|GetNS_CineticTrail) "speed" (Variables|Default|GetCurrentSpeed)))

(event Input|KeyboardEvents|DebugKeyS
  (params (Key :type Key%20Structure :default "None") (ActionValue :type Input%20Action%20Value%20Structure))
  (:Pressed
    (Variables|Default|SetPitchIncrement 1.0))
  (:Released
    (Variables|Default|SetPitchIncrement 0.0)))

(event Input|KeyboardEvents|DebugKeyA
  (params (Key :type Key%20Structure :default "None") (ActionValue :type Input%20Action%20Value%20Structure))
  (:Pressed
    (Variables|Default|SetRollIncrement 1.0))
  (:Released
    (Variables|Default|SetRollIncrement 0.0)))

(event Input|KeyboardEvents|DebugKeyQ
  (params (Key :type Key%20Structure :default "None") (ActionValue :type Input%20Action%20Value%20Structure))
  (:Pressed
    (Variables|Default|SetIncrement 1.0))
  (:Released
    (Variables|Default|SetIncrement 0.0)))

(event Input|KeyboardEvents|DebugKeyE
  (params (Key :type Key%20Structure :default "None") (ActionValue :type Input%20Action%20Value%20Structure))
  (:Pressed
    (Variables|Default|SetIncrement -1.0))
  (:Released
    (Variables|Default|SetIncrement 0.0)))

(event Input|KeyboardEvents|DebugKeyD
  (params (Key :type Key%20Structure :default "None") (ActionValue :type Input%20Action%20Value%20Structure))
  (:Pressed
    (Variables|Default|SetRollIncrement -1.0))
  (:Released
    (Variables|Default|SetRollIncrement 0.0)))

(event Input|KeyboardEvents|DebugKeyW
  (params (Key :type Key%20Structure :default "None") (ActionValue :type Input%20Action%20Value%20Structure))
  (:Pressed
    (Variables|Default|SetPitchIncrement -1.0))
  (:Released
    (Variables|Default|SetPitchIncrement 0.0)))

(fn ConstructionScript)