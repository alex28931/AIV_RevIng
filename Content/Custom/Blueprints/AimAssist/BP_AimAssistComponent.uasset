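; Aim assist component that nudges its owning pawn's view toward a target in front of a camera supplied through Init.
; Each tick it multi line-traces along the camera forward and picks the hit actor whose direction has the highest dot product above a threshold.
; It converts that direction to camera space and feeds scaled pitch and yaw into controller input.
; Debug trace drawing and screen prints are left on.
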(event `self.ReceiveBeginPlay`
  (bind _aspawn (cast `Pawn` (`self.GetOwner`)))
  (set `self.PawnOwner` _aspawn))

(event `self.ReceiveTick`
  (params (DeltaSeconds :type "Float (single-precision)"))
  (bind _ownercamera (`self.OwnerCamera`))
  (bind _pawnowner (`self.PawnOwner`))
  (bind _returnvalue (`SceneComponent.K2_GetComponentLocation` _ownercamera))
  (bind _returnvalue_2 (* (`GameplayStatics.GetWorldDeltaSeconds`) (`self.SpeedFactor`)))
  (bind (_returnvalue_roll _returnvalue_pitch _returnvalue_yaw) (`KismetMathLibrary.BreakRotator` (`KismetMathLibrary.MakeRotFromX` (`KismetMathLibrary.InverseTransformDirection` (`SceneComponent.K2_GetComponentToWorld` (`self.OwnerCamera`)) (`KismetMathLibrary.Normal` (- (`Actor.K2_GetActorLocation` (`self.BestHit`)) (`SceneComponent.K2_GetComponentLocation` (`self.OwnerCamera`))))))))
  (bind _outhits (`KismetSystemLibrary.LineTraceMulti` :`Start` _returnvalue :`End` (+ _returnvalue (* (`SceneComponent.GetForwardVector` _ownercamera) (`self.MaxDist`))) :`TraceChannel` "TraceTypeQuery4" :`DrawDebugType` "ForDuration"))
  (set `self.MaxDot` 0.0)
  (bind _output_get (set `self.HitActors` _outhits))
  (set `self.BestHit` null)
  (for _array_element _output_get
    (bind _returnvalue_3 (`KismetMathLibrary.Dot_VectorVector` (`SceneComponent.GetForwardVector` (`self.OwnerCamera`)) (`KismetMathLibrary.Normal` (- (`Actor.K2_GetActorLocation` (`.HitActor` (`GameplayStatics.BreakHitResult` _array_element))) (`SceneComponent.K2_GetComponentLocation` (`self.OwnerCamera`))))))
    (if (and (> _returnvalue_3 (`self.DotThreshold`)) (> _returnvalue_3 (`self.MaxDot`)))
      (set `self.MaxDot` _returnvalue_3)
      (set `self.BestHit` (`.HitActor` (`GameplayStatics.BreakHitResult` _array_element)))
      (`KismetSystemLibrary.PrintString` "ValidTarget" true true (struct :`G` 1.0 :`B` 0.072386 :`A` 1.0))
      (else
        (`KismetSystemLibrary.PrintString` "NoValidTargetFound" true true (struct :`R` 1.0 :`B` 0.01311 :`A` 1.0)))))
  (`/Engine/EditorBlueprintResources/StandardMacros.IsValid` (`self.BestHit`)
    (:`Is Valid`
      (bind _result (`/Engine/EditorBlueprintResources/StandardMacros.NegateFloat` (* _returnvalue_pitch _returnvalue_2))
        (:`  `
          (`Pawn.AddControllerPitchInput` _pawnowner _result)
          (`Pawn.AddControllerYawInput` _pawnowner (* _returnvalue_yaw _returnvalue_2)))))))

(fn `Init`
  (params (Camera :type "CameraComponent Object Reference"))
  (set `self.OwnerCamera` Camera))