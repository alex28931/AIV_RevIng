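; BPC_WidgetPointOfInterest is an unfinished component for tracking its owning actor as a point of interest on a minimap.
; BeginPlay caches the scene capture from the player's BP_MiniMapCharacter.
; Tick converts the player-to-owner offset into normalized coordinates using the capture's OrthoWidth, flipping Y, and tests whether they fall within map bounds.
; The bounds check triggers nothing; the widget slot positioning and pixel scaling are left unconnected.
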(event `self.ReceiveBeginPlay`
  (bind _asbp_mini_map_character (cast `/Game/Custom/Blueprints/MiniMap/BP_MiniMapCharacter` (`GameplayStatics.GetPlayerPawn` 0)))
  (set `self.SceneCapture2D` (`/Game/Custom/Blueprints/MiniMap/BP_MiniMapCharacter.SceneCaptureComponent2D` _asbp_mini_map_character)))

(event `self.ReceiveTick`
  (params (DeltaSeconds :type "Float (single-precision)"))
  (bind _orthowidth (`SceneCaptureComponent2D.OrthoWidth` (`self.SceneCapture2D`)))
  (bind _output_get (set `self.worldMapPosition` (- (`Actor.K2_GetActorLocation` (`GameplayStatics.GetPlayerPawn` 0)) (`Actor.K2_GetActorLocation` (`self.GetOwner`)))))
  (bind _returnvalue (+ (/ (.x _output_get) _orthowidth) 0.5))
  (bind _returnvalue_2 (- 1.0 (+ (/ (.y _output_get) _orthowidth) 0.5)))
  (if (and (> _returnvalue 0.0) (<= _returnvalue 1.0) (> _returnvalue_2 0.0) (<= _returnvalue_2 1.0))
    _))